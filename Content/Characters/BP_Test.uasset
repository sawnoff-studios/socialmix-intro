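; Test Blueprint that spins a cube and prints a door-state flag for debugging.
; BeginPlay prints DoorOpen, waits two seconds, sets it true and prints again through DebugDoorOpen, whose inputs and zero-vector outputs serve no function.
; Tick accumulates Angle from delta time and applies it as the cube's world yaw, independent of DoorOpen.
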(event EventBeginPlay
  (CallFunction|DebugDoorOpen 0.0 "0, 0, 0")
  (Utilities|FlowControl|Delay 2.0)
  (Variables|Default|SetDoorOpen true)
  (CallFunction|DebugDoorOpen 0.0 "0, 0, 0"))

(event Collision|EventActorBeginOverlap
  (params (OtherActor :type Actor%20Object%20Reference)))

(event EventTick
  (params (DeltaSeconds :type Float%20%28single-precision%29))
  (bind _output_get (Variables|Default|SetAngle (+ (* DeltaSeconds 2e+01) (Variables|Default|GetAngle))))
  (Transformation|SetWorldRotation (Variables|Default|GetCube) (Math|Rotator|MakeRotator 0.0 0.0 _output_get) false false))

(fn ConstructionScript)

(fn DebugDoorOpen
  (params (Test :type Float%20%28double-precision%29) (NewParam :type Vector))
  (Development|PrintString (Utilities|String|ToString(Text) (Utilities|Text|FormatText "Hello world the value of DoorOpen is {Door}" (Variables|Default|GetDoorOpen))) true true "(R=0.000000,G=0.660000,B=1.000000,A=1.000000)" 2e+02)
  (return "0, 0, 0" "0, 0, 0" "0, 0, 0"))